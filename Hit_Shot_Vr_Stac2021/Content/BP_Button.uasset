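; BP_Button is a pushable button actor that animates when anything overlaps its Box.
; An IsPushable gate starts a timeline offsetting Cube1 from the location cached at BeginPlay.
; When that finishes, it calls A (empty here), re-enables pushing and plays a second timeline on Cube1, so re-triggering is possible during that motion.
; Disconnected leftovers include a motion-controller cast and a MoveComponentTo version of the press.
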(event OnComponentBeginOverlap(Box)
  (params (OverlappedComponent :type Primitive%20Component%20Object%20Reference) (OtherActor :type Actor%20Object%20Reference) (OtherComp :type Primitive%20Component%20Object%20Reference) (OtherBodyIndex :type Integer) (bFromSweep :type Boolean) (SweepResult :type Hit%20Result%20Structure%20%28by%20ref%29))
  (if (Variables|Default|GetIsPushable)
    (Variables|Default|SetIsPushable false)
    (bind _새_트랙_0 (Timeline|타임라인_0 PlayFromStart)
      (:Update
        (Transformation|SetRelativeLocation (Variables|Default|GetCube1) (+ (* _새_트랙_0 -1e+02) (Variables|Default|GetButtonPos)) false false))
      (:Finished
        (CallFunction|A)
        (Variables|Default|SetIsPushable true)
        (bind _새_트랙_0_2 (Timeline|타임라인_1 PlayFromStart)
          (:Update
            (Transformation|SetRelativeLocation (Variables|Default|GetCube1) (+ (* _새_트랙_0_2 -1e+02) (Variables|Default|GetButtonPos)) false false)))))))

(event EventBeginPlay
  (Variables|Default|SetButtonPos (Variables|/Script/Engine.SceneComponent|GetRelativeLocation (Variables|Default|GetCube1))))

(event Collision|EventActorBeginOverlap
  (params (OtherActor :type Actor%20Object%20Reference)))

(event EventTick
  (params (DeltaSeconds :type Float%20%28single-precision%29)))

(fn ConstructionScript)

(fn A)